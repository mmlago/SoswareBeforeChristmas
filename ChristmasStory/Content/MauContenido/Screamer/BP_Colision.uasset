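; BP_Colision is a trigger volume that, judging by its Screamer folder, stages a jump scare for the first-person player.
; When BP_FirstPersonCharacter enters the Box, it plays an explosion sound and starts a short timer that spawns BP_Character at the Box location.
; After a brief delay it destroys both the spawned character and itself, while the end-overlap handler only casts and does nothing further.
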(event `self.Box.OnComponentBeginOverlap`
  (params (OverlappedComponent :type "PrimitiveComponent Object Reference") (OtherActor :type "Actor Object Reference") (OtherComp :type "PrimitiveComponent Object Reference") (OtherBodyIndex :type Integer) (bFromSweep :type Boolean) (SweepResult :type "HitResult Structure (by ref)"))
  (cast `/Game/FirstPerson/Blueprints/BP_FirstPersonCharacter` OtherActor)
  (if true
    (`KismetSystemLibrary.K2_SetTimerDelegate` (delegate `SpawnCharacter`) 0.1)
    (`GameplayStatics.PlaySound2D` "/Game/StarterContent/Audio/Explosion01.Explosion01" 1.0 1.0 0.0 null null)))

(event `SpawnCharacter`
  (bind _returnvalue (`|SpawnActorFromClass` "/Game/MauContenido/Characters/Muerto/BP_Character.BP_Character_C" (`KismetMathLibrary.MakeTransform` (`SceneComponent.K2_GetComponentLocation` (`self.Box`))) "Undefined" "MultiplyWithRoot" null null))
  (bind _asbp_character (cast `/Game/MauContenido/Characters/Muerto/BP_Character` _returnvalue))
  (`KismetSystemLibrary.Delay` 1.0)
  (`self.K2_DestroyActor` _asbp_character)
  (`self.K2_DestroyActor` self))

(event `self.Box.OnComponentEndOverlap`
  (params (OverlappedComponent :type "PrimitiveComponent Object Reference") (OtherActor :type "Actor Object Reference") (OtherComp :type "PrimitiveComponent Object Reference") (OtherBodyIndex :type Integer))
  (cast `/Game/FirstPerson/Blueprints/BP_FirstPersonCharacter` OtherActor))

(fn `UserConstructionScript`)